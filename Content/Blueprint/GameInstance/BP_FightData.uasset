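; BP_FightData stores the width and height of a fight board and exposes events to adjust them.
; Separate events raise or lower each dimension by one, with no limits applied.
; ShowBoardSize prints the current width and height to the screen as a comma-separated pair for debugging.
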(event `WidthPlus`
  (set `self.BoardWidth` (+ (`self.BoardWidth`) 1)))

(event `WidthMinus`
  (set `self.BoardWidth` (+ (`self.BoardWidth`) -1)))

(event `HeightPlus`
  (set `self.BoardHeight` (+ (`self.BoardHeight`) 1)))

(event `ShowBoardSize`
  (`KismetSystemLibrary.PrintString` (`KismetStringLibrary.Concat_StrStr` (`KismetStringLibrary.Conv_IntToString` (`self.BoardWidth`)) ", " (`KismetStringLibrary.Conv_IntToString` (`self.BoardHeight`)))))

(event `HeightMinus`
  (set `self.BoardHeight` (+ (`self.BoardHeight`) -1)))