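; Enemy melee attack gameplay ability that damages the avatar's combat target.
; On activation it gets the target through a combat message, requires the avatar to implement CombatInterface, then calls CauseDamage and ends immediately.
; Disconnected logic holds a random tagged montage waiting on its gameplay event, and a radius-based area attack on live players around a combat socket; neither runs.
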(event `self.K2_ActivateAbility`
  (bind _returnvalue (`self.GetAvatarActorFromActorInfo`))
  (bind _returnvalue_2 (message `EnemyInterface.GetCombatTarget` _returnvalue))
  (bind _ascombat_interface (cast `CombatInterface` _returnvalue))
  (`self.CauseDamage` _returnvalue_2)
  (`self.K2_EndAbility`))