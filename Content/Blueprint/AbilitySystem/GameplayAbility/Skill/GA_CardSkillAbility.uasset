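; GA_CardSkillAbility is a gameplay ability for card-driven skills, with shared activation, montage and cleanup logic.
; On activation it caches the avatar's ZAttributeSet and the card component's ActivatingCard, then hides the player's skill range display.
; A PlayMontage event plays AbilityMontage and begins waiting for the Montage.Attack.Weapon gameplay event, with no follow-up wired here.
; When the ability ends, it reduces weapon durability if WeaponTag is valid.
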(event `self.K2_ActivateAbility`
  (bind _returnvalue (`AbilitySystemComponent.GetAttributeSet` (`AbilitySystemBlueprintLibrary.GetAbilitySystemComponent` (`self.GetAvatarActorFromActorInfo`)) "/Script/ProjectZ.ZAttributeSet"))
  (bind _aszattribute_set (cast `ZAttributeSet` _returnvalue))
  (set `self.AttributeSet` _aszattribute_set)
  (bind _aszplayer_character (cast `ZPlayerCharacter` (`self.GetAvatarActorFromActorInfo`)))
  (bind _output_get (set `self.CardComponent` (`ZCharacterBase.GetCardComponent` _aszplayer_character)))
  (set `self.ActivatingCard` (`CardComponent.ActivatingCard` _output_get))
  (bind _aszplayer_character_2 (cast `ZPlayerCharacter` (`self.GetAvatarActorFromActorInfo`)))
  (`ZPlayerCharacter.HideSkillRange` _aszplayer_character_2))

(event `self.K2_OnEndAbility`
  (params (bWasCancelled :type Boolean))
  (if (`BlueprintGameplayTagLibrary.IsGameplayTagValid` (`self.WeaponTag`))
    (`self.ReduceWeaponDurability` (`self.WeaponTag`))))

(event `PlayMontage`
  (`AbilityTask_PlayMontageAndWait.CreatePlayMontageAndWaitProxy` "None" (`self.AbilityMontage`) 1.0 "None" false
    (:`then`
      (`AbilityTask_WaitGameplayEvent.WaitGameplayEvent` (struct :`TagName` "Montage.Attack.Weapon") null))))