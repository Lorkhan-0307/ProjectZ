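; GA_Salt is a card-driven gameplay ability that damages bleeding characters in a sector in front of the caster, aimed at the mouse.
; On activation it gets the target data under the mouse, then gathers actors in that sector using the card's skill angle and range, excluding the avatar.
; Each character hit takes damage equal to its bleed count multiplied by Dexterity plus card level plus one, then the ability ends.
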(event `self.K2_ActivateAbility`
  (bind _returnvalue (`self.GetAvatarActorFromActorInfo`))
  (bind (_activatingcard_cardname _activatingcard_cardbackgroundimage _activatingcard_cardimage _activatingcard_cardcost _activatingcard_cardatk _activatingcard_carddef _activatingcard_carddescription _activatingcard_cardtype _activatingcard_cardlevel _activatingcard_skillrange _activatingcard_skillangle) (break `Card` (`self.ActivatingCard`)))
  (bind (_activatingcard_cardname_2 _activatingcard_cardbackgroundimage_2 _activatingcard_cardimage_2 _activatingcard_cardcost_2 _activatingcard_cardatk_2 _activatingcard_carddef_2 _activatingcard_carddescription_2 _activatingcard_cardtype_2 _activatingcard_cardlevel_2) (break `Card` (`self.ActivatingCard`)))
  (bind (_dexterity_basevalue _dexterity_currentvalue) (break `GameplayAttributeData` (`ZAttributeSet.Dexterity` (`self.AttributeSet`))))
  (`parent.K2_ActivateAbility`)
  (bind (_asynctaskproxy _data) (`TargetDataUnderMouse.CreateTargetDataUnderMouse`)
    (:`then`
      (bind _outoverlappingactors (`ZAbilitySystemLibrary.GetSectorFormTarget` _returnvalue (`|MakeArray` _returnvalue) _activatingcard_skillangle _activatingcard_skillrange (`Actor.K2_GetActorLocation` _returnvalue) (`.Location` (`GameplayStatics.BreakHitResult` _data))))
      (for _array_element _outoverlappingactors
        (bind _aszcharacter_base (cast `ZCharacterBase` _array_element))
        (set `self.Damage` (* (`ZCharacterBase.BleedCount` _aszcharacter_base) (+ _dexterity_currentvalue _activatingcard_cardlevel_2 1.0)))
        (`self.CauseDamage` _array_element))
      (`self.K2_EndAbility`))))