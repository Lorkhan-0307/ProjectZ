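; Gameplay ability for the Blocking card skill, which grants defence to the avatar character.
; On activation it reads the Blocking row from DT_Card and adds defence equal to the card's CardAtk value plus the Strength attribute and the activating card's level.
; It then calls PlayMontage and immediately ends the ability.
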(event `self.K2_ActivateAbility`
  (bind (_strength_basevalue _strength_currentvalue) (break `GameplayAttributeData` (`ZAttributeSet.Strength` (`self.AttributeSet`))))
  (`parent.K2_ActivateAbility`)
  (bind _returnvalue (`|GetDataTableRow` "/Game/Blueprint/Data/DT_Card.DT_Card" "Blocking")
    (:`then`
      (bind _aszcharacter_base (cast `ZCharacterBase` (`self.GetAvatarActorFromActorInfo`)))
      (bind (_activatingcard_cardname _activatingcard_cardbackgroundimage _activatingcard_cardimage _activatingcard_cardcost _activatingcard_cardatk _activatingcard_carddef _activatingcard_carddescription _activatingcard_cardtype _activatingcard_cardlevel) (break `Card` (`CardComponent.ActivatingCard` (`ZCharacterBase.GetCardComponent` _aszcharacter_base))))
      (`ZAttributeSet.AddDefenceInBlueprint` (`self.AttributeSet`) (+ (+ (`.CardAtk` (break `Card` _returnvalue)) _strength_currentvalue) _activatingcard_cardlevel))
      (`self.PlayMontage`)
      (`self.K2_EndAbility`))))