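; GA_Frenzy is a card-driven skill gameplay ability that sets buff values and targets its own avatar.
; On activation it derives buff magnitude from the activating card's attack plus level, and buff duration from its defense, extended at level three.
; It then passes the avatar to CauseDamage, which is defined outside this graph, and ends immediately.
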(event `self.K2_ActivateAbility`
  (bind (_activatingcard_cardname _activatingcard_cardbackgroundimage _activatingcard_cardimage _activatingcard_cardcost _activatingcard_cardatk _activatingcard_carddef _activatingcard_carddescription _activatingcard_cardtype _activatingcard_cardlevel) (break `Card` (`CardComponent.ActivatingCard` (`self.CardComponent`))))
  (`parent.K2_ActivateAbility`)
  (set `self.BuffMagnitude` (+ _activatingcard_cardatk _activatingcard_cardlevel))
  (if (== _activatingcard_cardlevel 3)
    (set `self.BuffDuration` (+ _activatingcard_carddef 1))
    (else
      (set `self.BuffDuration` _activatingcard_carddef)))
  (`self.CauseDamage` (`self.GetAvatarActorFromActorInfo`))
  (`self.K2_EndAbility`))