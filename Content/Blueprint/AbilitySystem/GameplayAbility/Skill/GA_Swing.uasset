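; GA_Swing is a card-driven skill ability that hits targets in a sector in front of the avatar, aimed at the point under the mouse.
; A target-data task supplies the mouse location, and the active card sets the sector's angle and range.
; Damage from card defense, card level and Strength is floored after being split across all targets hit.
; Debuff chance comes from Strength, card attack and card level.
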(event `self.K2_ActivateAbility`
  (bind _returnvalue (`self.GetAvatarActorFromActorInfo`))
  (bind (_activatingcard_cardname _activatingcard_cardbackgroundimage _activatingcard_cardimage _activatingcard_cardcost _activatingcard_cardatk _activatingcard_carddef _activatingcard_carddescription _activatingcard_cardtype _activatingcard_cardlevel _activatingcard_skillrange _activatingcard_skillangle) (break `Card` (`self.ActivatingCard`)))
  (bind (_activatingcard_cardname_2 _activatingcard_cardbackgroundimage_2 _activatingcard_cardimage_2 _activatingcard_cardcost_2 _activatingcard_cardatk_2 _activatingcard_carddef_2 _activatingcard_carddescription_2 _activatingcard_cardtype_2 _activatingcard_cardlevel_2) (break `Card` (`self.ActivatingCard`)))
  (bind (_activatingcard_cardname_3 _activatingcard_cardbackgroundimage_3 _activatingcard_cardimage_3 _activatingcard_cardcost_3 _activatingcard_cardatk_3 _activatingcard_carddef_3 _activatingcard_carddescription_3 _activatingcard_cardtype_3 _activatingcard_cardlevel_3) (break `Card` (`self.ActivatingCard`)))
  (bind (_strength_basevalue _strength_currentvalue) (break `GameplayAttributeData` (`ZAttributeSet.Strength` (`self.AttributeSet`))))
  (bind (_strength_basevalue_2 _strength_currentvalue_2) (break `GameplayAttributeData` (`ZAttributeSet.Strength` (`self.AttributeSet`))))
  (`parent.K2_ActivateAbility`)
  (set `self.DebuffChance` (+ (* _strength_currentvalue 10.0) _activatingcard_cardatk_2 (* _activatingcard_cardlevel_2 10)))
  (bind (_asynctaskproxy _data) (`TargetDataUnderMouse.CreateTargetDataUnderMouse`)
    (:`then`
      (bind _outoverlappingactors (`ZAbilitySystemLibrary.GetSectorFormTarget` _returnvalue (`|MakeArray` _returnvalue) _activatingcard_skillangle _activatingcard_skillrange (`Actor.K2_GetActorLocation` _returnvalue) (`.Location` (`GameplayStatics.BreakHitResult` _data))))
      (for _array_element _outoverlappingactors
        (set `self.Damage` (`KismetMathLibrary.Conv_IntToDouble` (`KismetMathLibrary.FFloor` (/ (+ _activatingcard_carddef_3 _strength_currentvalue_2 _activatingcard_cardlevel_3) (`KismetArrayLibrary.Array_Length` _outoverlappingactors)))))
        (`self.CauseDamage` _array_element))
      (`self.K2_EndAbility`))))