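; Smash skill ability that hits the actor under the mouse with a weapon attack.
; Once target data arrives, it computes Damage from weapon attack, Strength and the activating card's level, and adds Strength and card-level bonuses onto the existing DebuffChance.
; It then plays the ability montage and waits for the Montage.Attack.Weapon gameplay event to cause damage to the target and end the ability.
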(event `self.K2_ActivateAbility`
  (bind _attributeset (`self.AttributeSet`))
  (bind (_strength_basevalue _strength_currentvalue) (break `GameplayAttributeData` (`ZAttributeSet.Strength` (`self.AttributeSet`))))
  (bind (_activatingcard_cardname _activatingcard_cardbackgroundimage _activatingcard_cardimage _activatingcard_cardcost _activatingcard_cardatk _activatingcard_carddef _activatingcard_carddescription _activatingcard_cardtype _activatingcard_cardlevel) (break `Card` (`CardComponent.ActivatingCard` (`self.CardComponent`))))
  (bind (_weaponatk_basevalue _weaponatk_currentvalue) (break `GameplayAttributeData` (`ZAttributeSet.WeaponAtk` _attributeset)))
  (bind (_strength_basevalue_2 _strength_currentvalue_2) (break `GameplayAttributeData` (`ZAttributeSet.Strength` _attributeset)))
  (`parent.K2_ActivateAbility`)
  (bind (_asynctaskproxy _data) (`TargetDataUnderMouse.CreateTargetDataUnderMouse`)
    (:`then`
      (set `self.Data Hit Actor` (`.HitActor` (`GameplayStatics.BreakHitResult` _data)))
      (set `self.DebuffChance` (+ (`self.DebuffChance`) (* _strength_currentvalue 10.0) (* _activatingcard_cardlevel 10)))
      (set `self.Damage` (+ _weaponatk_currentvalue (* _strength_currentvalue_2 2.0) _activatingcard_cardlevel))
      (`AbilityTask_PlayMontageAndWait.CreatePlayMontageAndWaitProxy` "None" (`self.AbilityMontage`) 1.0 "None" false
        (:`then`
          (`AbilityTask_WaitGameplayEvent.WaitGameplayEvent` (struct :`TagName` "Montage.Attack.Weapon") null
            (:`EventReceived`
              (`self.CauseDamage` (`self.Data Hit Actor`))
              (`self.K2_EndAbility`))))))))