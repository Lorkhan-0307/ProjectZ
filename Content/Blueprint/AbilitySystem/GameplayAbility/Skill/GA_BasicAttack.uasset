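; Basic attack gameplay ability that damages the actor under the mouse using the activating card's attack value.
; A target-data-under-mouse task supplies the hit actor, and the card's attack becomes the damage.
; The card type selects a one- or two-hand weapon tag, with only one-hand setting a guaranteed debuff chance, before CauseDamage runs.
; The ability ends after damage or when the target is invalid.
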(event `self.K2_ActivateAbility`
  (bind (_activatingcard_cardname _activatingcard_cardbackgroundimage _activatingcard_cardimage _activatingcard_cardcost _activatingcard_cardatk _activatingcard_carddef _activatingcard_carddescription _activatingcard_cardtype) (break `Card` (`CardComponent.ActivatingCard` (`self.CardComponent`))))
  (`parent.K2_ActivateAbility`)
  (bind (_asynctaskproxy _data) (`TargetDataUnderMouse.CreateTargetDataUnderMouse`)
    (:`then`
      (set `self.Data Hit Actor` (`.HitActor` (`GameplayStatics.BreakHitResult` _data)))
      (set `self.Damage` (`KismetMathLibrary.Conv_IntToDouble` _activatingcard_cardatk))
      (`/Engine/EditorBlueprintResources/StandardMacros.IsValid` (`self.Data Hit Actor`)
        (:`Is Valid`
          (switch `ECardType` _activatingcard_cardtype
            (:`ECT_OneHandWeapon`
              (set `self.WeaponTag` (struct :`TagName` "Card.Weapon.OneHand"))
              (set `self.DebuffChance` 100.0))
            (:`ECT_TwoHandWeapon`
              (set `self.WeaponTag` (struct :`TagName` "Card.Weapon.TwoHand"))))
          (`self.CauseDamage` (`self.Data Hit Actor`)))
        (:`Is Not Valid`
          _))
      (`self.K2_EndAbility`))))