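; GA_Block is a card skill gameplay ability that grants Defence to the avatar ZCharacterBase.
; On activation it adds the activating card's attack value, the Strength attribute and the card level to Defence, then plays the ability montage.
; The ability ends on the Montage.Attack.Weapon gameplay event rather than on montage completion, and the montage keeps playing afterwards.
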(event `self.K2_ActivateAbility`
  (bind (_strength_basevalue _strength_currentvalue) (break `GameplayAttributeData` (`ZAttributeSet.Strength` (`self.AttributeSet`))))
  (bind (_activatingcard_cardname _activatingcard_cardbackgroundimage _activatingcard_cardimage _activatingcard_cardcost _activatingcard_cardatk) (break `Card` (`CardComponent.ActivatingCard` (`self.CardComponent`))))
  (`parent.K2_ActivateAbility`)
  (bind _aszcharacter_base (cast `ZCharacterBase` (`self.GetAvatarActorFromActorInfo`)))
  (bind (_activatingcard_cardname_2 _activatingcard_cardbackgroundimage_2 _activatingcard_cardimage_2 _activatingcard_cardcost_2 _activatingcard_cardatk_2 _activatingcard_carddef _activatingcard_carddescription _activatingcard_cardtype _activatingcard_cardlevel) (break `Card` (`CardComponent.ActivatingCard` (`ZCharacterBase.GetCardComponent` _aszcharacter_base))))
  (`ZAttributeSet.AddDefenceInBlueprint` (`self.AttributeSet`) (+ (+ _activatingcard_cardatk _strength_currentvalue) _activatingcard_cardlevel))
  (`AbilityTask_PlayMontageAndWait.CreatePlayMontageAndWaitProxy` "None" (`self.AbilityMontage`) 1.0 "None" false
    (:`then`
      (`AbilityTask_WaitGameplayEvent.WaitGameplayEvent` (struct :`TagName` "Montage.Attack.Weapon") null
        (:`EventReceived`
          (`self.K2_EndAbility`))))))