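; Stab card skill ability that detonates a target's Bleed, turning its bleed count into damage.
; It takes the character under the mouse and multiplies BleedCount by the sum of weapon attack, dexterity and card level.
; The ability montage plays, and its Montage.Attack.Weapon gameplay event applies the damage, removes the Bleed debuff and ends the ability.
; A target that is not a ZCharacterBase halts the flow without calling EndAbility.
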(event `self.K2_ActivateAbility`
  (bind _attributeset (`self.AttributeSet`))
  (bind (_activatingcard_cardname _activatingcard_cardbackgroundimage _activatingcard_cardimage _activatingcard_cardcost _activatingcard_cardatk _activatingcard_carddef _activatingcard_carddescription _activatingcard_cardtype _activatingcard_cardlevel) (break `Card` (`CardComponent.ActivatingCard` (`self.CardComponent`))))
  (bind (_weaponatk_basevalue _weaponatk_currentvalue) (break `GameplayAttributeData` (`ZAttributeSet.WeaponAtk` _attributeset)))
  (bind (_dexterity_basevalue _dexterity_currentvalue) (break `GameplayAttributeData` (`ZAttributeSet.Dexterity` _attributeset)))
  (`parent.K2_ActivateAbility`)
  (bind (_asynctaskproxy _data) (`TargetDataUnderMouse.CreateTargetDataUnderMouse`)
    (:`then`
      (bind _output_get (set `self.TargetActor` (`.HitActor` (`GameplayStatics.BreakHitResult` _data))))
      (bind _aszcharacter_base (cast `ZCharacterBase` _output_get))
      (set `self.Damage` (* (`KismetMathLibrary.Conv_IntToDouble` (`ZCharacterBase.BleedCount` _aszcharacter_base)) (+ _weaponatk_currentvalue _dexterity_currentvalue _activatingcard_cardlevel)))
      (`AbilityTask_PlayMontageAndWait.CreatePlayMontageAndWaitProxy` "None" (`self.AbilityMontage`) 1.0 "None" false
        (:`then`
          (`AbilityTask_WaitGameplayEvent.WaitGameplayEvent` (struct :`TagName` "Montage.Attack.Weapon") null
            (:`EventReceived`
              (`self.CauseDamage` (`self.TargetActor`))
              (bind _ascombat_interface (cast `CombatInterface` (`self.TargetActor`)))
              (`CombatInterface.RemoveDebuff` _ascombat_interface (struct :`TagName` "Debuff.Bleed"))
              (`self.K2_EndAbility`))))))))