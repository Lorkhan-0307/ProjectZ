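; GA_Wound is a card skill gameplay ability that damages the actor under the mouse.
; On activation, a TargetDataUnderMouse node supplies the hit actor as the target.
; It sets DebuffStack to the activating card's attack plus level, read from CardComponent, then calls CauseDamage on the target and ends.
; The damage and debuff logic itself lives outside this graph.
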(event `self.K2_ActivateAbility`
  (bind (_activatingcard_cardname _activatingcard_cardbackgroundimage _activatingcard_cardimage _activatingcard_cardcost _activatingcard_cardatk _activatingcard_carddef _activatingcard_carddescription _activatingcard_cardtype _activatingcard_cardlevel) (break `Card` (`CardComponent.ActivatingCard` (`self.CardComponent`))))
  (`parent.K2_ActivateAbility`)
  (bind (_asynctaskproxy _data) (`TargetDataUnderMouse.CreateTargetDataUnderMouse`)
    (:`then`
      (set `self.TargetActor` (`.HitActor` (`GameplayStatics.BreakHitResult` _data)))
      (set `self.DebuffStack` (+ _activatingcard_cardatk _activatingcard_cardlevel))
      (`self.CauseDamage` (`self.TargetActor`))
      (`self.K2_EndAbility`))))