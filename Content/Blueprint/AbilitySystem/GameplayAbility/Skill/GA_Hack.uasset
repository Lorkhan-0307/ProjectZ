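; GA_Hack is a gameplay ability for a card-driven melee weapon skill against the actor under the mouse.
; On activation it captures that hit actor, then plays the ability montage.
; When the montage sends the weapon-attack gameplay event, it computes damage from weapon attack, Dexterity and the activating card's level and attack, applies it to the target, and ends the ability.
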(event `self.K2_ActivateAbility`
  (bind (_activatingcard_cardname _activatingcard_cardbackgroundimage _activatingcard_cardimage _activatingcard_cardcost _activatingcard_cardatk _activatingcard_carddef _activatingcard_carddescription _activatingcard_cardtype _activatingcard_cardlevel) (break `Card` (`self.ActivatingCard`)))
  (bind _attributeset (`self.AttributeSet`))
  (bind (_weaponatk_basevalue _weaponatk_currentvalue) (break `GameplayAttributeData` (`ZAttributeSet.WeaponAtk` _attributeset)))
  (bind (_dexterity_basevalue _dexterity_currentvalue) (break `GameplayAttributeData` (`ZAttributeSet.Dexterity` _attributeset)))
  (`parent.K2_ActivateAbility`)
  (bind (_asynctaskproxy _data) (`TargetDataUnderMouse.CreateTargetDataUnderMouse`)
    (:`then`
      (set `self.Data Hit Actor` (`.HitActor` (`GameplayStatics.BreakHitResult` _data)))
      (`AbilityTask_PlayMontageAndWait.CreatePlayMontageAndWaitProxy` "None" (`self.AbilityMontage`) 1.0 "None" false
        (:`then`
          (`AbilityTask_WaitGameplayEvent.WaitGameplayEvent` (struct :`TagName` "Montage.Attack.Weapon") null
            (:`EventReceived`
              (set `self.Damage` (* (+ _weaponatk_currentvalue _dexterity_currentvalue _activatingcard_cardlevel) _activatingcard_cardatk))
              (`self.CauseDamage` (`self.Data Hit Actor`))
              (`self.K2_EndAbility`))))))))