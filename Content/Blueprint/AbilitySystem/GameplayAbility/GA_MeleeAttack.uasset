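; Melee attack gameplay ability, currently a debug stub that finds nearby targets but applies no damage.
; On activation it queries the avatar's combat target, requires CombatInterface, then finds live players within a small radius, excluding itself.
; It draws a debug sphere on each one and ends immediately.
; The montage and gameplay-event wait that would time the hit check are disconnected and never run.
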(event `self.K2_ActivateAbility`
  (bind _returnvalue (`self.GetAvatarActorFromActorInfo`))
  (bind _returnvalue_2 (`self.GetAvatarActorFromActorInfo`))
  (message `EnemyInterface.GetCombatTarget` _returnvalue_2)
  (cast `CombatInterface` _returnvalue_2)
  (bind _outoverlappingactors (`ZAbilitySystemLibrary.GetLivePlayersWithinRadius` _returnvalue (`|MakeArray` _returnvalue) 200.0 (`Actor.K2_GetActorLocation` _returnvalue)))
  (for _array_element _outoverlappingactors
    (`KismetSystemLibrary.DrawDebugSphere` (`Actor.K2_GetActorLocation` _array_element) 30.0 12 (struct :`R` 1.0 :`G` 0.877511 :`A` 1.0) 1.0))
  (`self.K2_EndAbility`))