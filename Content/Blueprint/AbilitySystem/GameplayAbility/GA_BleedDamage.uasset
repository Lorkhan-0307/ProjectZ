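; GA_BleedDamage is a Gameplay Ability that deals bleed damage to its own avatar.
; On activation it sets damage to twice the ZCharacterBase bleed count and applies it through CauseDamage.
; It then removes the Bleed debuff through the avatar's CombatInterface and ends.
; A failed cast to either type stops the flow before EndAbility is called.
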(event `self.K2_ActivateAbility`
  (bind _aszcharacter_base (cast `ZCharacterBase` (`self.GetAvatarActorFromActorInfo`)))
  (set `self.Damage` (`KismetMathLibrary.Conv_IntToDouble` (* (`ZCharacterBase.BleedCount` _aszcharacter_base) 2)))
  (`self.CauseDamage` (`self.GetAvatarActorFromActorInfo`))
  (bind _ascombat_interface (cast `CombatInterface` (`self.GetAvatarActorFromActorInfo`)))
  (`CombatInterface.RemoveDebuff` _ascombat_interface (struct :`TagName` "Debuff.Bleed"))
  (`self.K2_EndAbility`))