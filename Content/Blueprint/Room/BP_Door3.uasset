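; BP_Door3 is an interactable door that moves the player through it by teleporting rather than opening.
; On Interact, it compares the player's distance to the Left and Right components and teleports the player to the farther one with zeroed rotation.
; An unconnected branch that would toggle the door's Pawn collision between Block and Overlap based on its relative yaw never runs.
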(event `self.ReceiveTick`
  (params (DeltaSeconds :type "Float (single-precision)")))

(event `self.Interact`
  (params (Player :type "Actor Object Reference"))
  (bind _returnvalue (`SceneComponent.K2_GetComponentLocation` (`Actor.RootComponent` Player)))
  (if (> (`KismetMathLibrary.Vector_Distance` _returnvalue (`SceneComponent.K2_GetComponentLocation` (`self.Left`))) (`KismetMathLibrary.Vector_Distance` _returnvalue (`SceneComponent.K2_GetComponentLocation` (`self.Right`))))
    (`self.K2_TeleportTo` :`self` Player :`DestLocation` (`SceneComponent.K2_GetComponentLocation` (`self.Left`)))
    (else
      (`self.K2_TeleportTo` :`self` Player :`DestLocation` (`SceneComponent.K2_GetComponentLocation` (`self.Right`))))))

(fn `UserConstructionScript`)